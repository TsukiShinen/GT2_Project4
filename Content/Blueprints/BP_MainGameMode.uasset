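; Main game mode that manages player checkpoint respawns, game over with level reload, and enemy spawn and kill tracking.
; A looping timer checks the grounded player against cached NavMeshBoundsVolumes, updating their current volume and firing a notification when they leave it.
; Registered enemies are assigned their containing volume, and unregistering prints a victory message once no spawners remain and kills equal spawns.
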(event Custom|UpdateCheckPoint
  (params (CheckPointOverlapped :type BP%20Check%20Point%20Object%20Reference))
  (Variables|Default|SetLastCheckPointOverlapped CheckPointOverlapped))

(event Custom|RespawnPlayer
  (bind _lastcheckpointoverlapped (Variables|Default|GetLastCheckPointOverlapped))
  (bind _returnvalue (Default|GetCheckPointRespawnTransform _lastcheckpointoverlapped))
  ;[1 1 1] RespawnPlayer
  (Utilities|IsValid _lastcheckpointoverlapped
    (:Is%20Valid
      (Transformation|SetActorLocation (Game|Player|GetPlayerPawn 0) (.location _returnvalue) false false)
      (Pawn|SetControlRotation (Game|GetPlayerController 0) (.rotation _returnvalue))
      (Default|UpdateLife (Variables|Default|GetPlayer) (Variables|Default|GetLifeDamageAfterRespawn)))))

(event Custom|GameOver
  (Development|PrintString "Game Over..." true true "(R=1.000000,G=0.000000,B=0.000000,A=1.000000)")
  (Utilities|FlowControl|Delay 2.0)
  (Game|OpenLevel(byObjectReference) "/Game/Maps/MainLevel.MainLevel"))

(event Custom|RegisterEnemy
  (params (NewEnemy :type BP%20Base%20Enemy%20Object%20Reference))
  (Utilities|Array|AddUnique (Variables|Default|GetEnemies) NewEnemy)
  (Math|Integer|IncrementInt (Variables|Default|GetEnemiesSpawned)
    (:%20%20
      (bind _array_element (Utilities|Array|ForEachLoopwithBreak (Variables|Default|GetNavMeshVolumes) :!label _label)
        (:LoopBody
          (bind _result (CallFunction|IsCharacteronNavMesh NewEnemy _array_element))
          (if _result
            (Variables|/Game/Blueprints/Enemies/BP_BaseEnemy.BP_BaseEnemy_C|SetcurrentNavMesh NewEnemy _array_element)
            (goto _label Break)))))))

(event Custom|RegisterPlayer
  (bind _returnvalue (Actor|GetActorOfClass "/Game/FirstPersonBP/Blueprints/FirstPersonCharacter.FirstPersonCharacter_C"))
  (Variables|Default|SetPlayer _returnvalue))

(event Custom|UnregisterEnemy
  (params (KilledEnemy :type BP%20Base%20Enemy%20Object%20Reference))
  (bind _returnvalue (Utilities|Array|RemoveItem (Variables|Default|GetEnemies) KilledEnemy))
  (if _returnvalue
    (Math|Integer|IncrementInt (Variables|Default|GetEnemiesKilled)
      (:%20%20
        (bind _outactors (Actor|GetAllActorsOfClass "/Game/Blueprints/BP_EnemySpawner.BP_EnemySpawner_C")) ; Not perfect, just for the test
        (if (and (== (Utilities|Array|Length _outactors) 0) (== (Variables|Default|GetEnemiesKilled) (Variables|Default|GetEnemiesSpawned)))
          (Development|PrintString "You killed all the enemies !" true true "(R=1.000000,G=0.145191,B=0.000000,A=1.000000)"))))
    (else
      (Development|PrintString "Try to remove an enemy who hasn't been registered..." true true "(R=1.000000,G=0.000000,B=0.000000,A=1.000000)" 3.0))))

(event Custom|CheckPlayerOnNavMesh
  (bind _player (Variables|Default|GetPlayer))
  (Utilities|IsValid _player
    (:Is%20Valid
      (if (AI|Components|NavMovement|IsMovingonGround (Variables|/Script/Engine.Character|GetCharacterMovement _player))
        (bind _result (CallFunction|IsCharacteronNavMesh (Variables|Default|GetPlayer) (Variables|/Game/FirstPersonBP/Blueprints/FirstPersonCharacter.FirstPersonCharacter_C|GetCurrentNavMesh _player)))
        (if (not _result)
          (CallFunction|CheckonAllNavMeshVolumes))))))

(event EventBeginPlay
  ;[1 1 1] Init data
  (CallFunction|RegisterPlayer)
  (bind _outactors (Actor|GetAllActorsOfClass "/Script/NavigationSystem.NavMeshBoundsVolume"))
  (Variables|Default|SetNavMeshVolumes _outactors)
  (Utilities|Time|SetTimerbyEvent (delegate Custom|CheckPlayerOnNavMesh) 1.0 true))

(fn ConstructionScript)

(fn CheckonAllNavMeshVolumes
  (bind _array_element (Utilities|Array|ForEachLoopwithBreak (Variables|Default|GetNavMeshVolumes) :!label _label)
    (:LoopBody
      (bind _result (CallFunction|IsCharacteronNavMesh (Variables|Default|GetPlayer) _array_element))
      (bind _output_get (LocalVariables|SetIsOverlappingOne _result))
      (if _output_get
        (Variables|/Game/FirstPersonBP/Blueprints/FirstPersonCharacter.FirstPersonCharacter_C|SetCurrentNavMesh (Variables|Default|GetPlayer) _array_element)
        (Default|CallOnPlayerIsOverlappingNewNavMesh)
        (goto _label Break)))
    (:Completed
      ;[1 1 1] If the player is not above a navMeshVolume, currentNavMesh = null
      (if (not (LocalVariables|GetIsOverlappingOne))
        (Variables|/Game/FirstPersonBP/Blueprints/FirstPersonCharacter.FirstPersonCharacter_C|SetCurrentNavMesh (Variables|Default|GetPlayer) 0)
        (Default|CallOnPlayerIsOverlappingNewNavMesh)))))