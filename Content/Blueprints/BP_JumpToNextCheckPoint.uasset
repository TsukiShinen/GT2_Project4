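; Debug-style helper actor that lets the local player hop between checkpoints by pressing N.
; It enables input for player controller 0 on BeginPlay and acts only when its CheckPoints array holds at least two entries.
; Each press advances a wrapping index, moves the pawn slightly above that checkpoint's arrow component and sets control rotation from the checkpoint's respawn transform.
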(event EventBeginPlay
  (Input|EnableInput (Game|GetPlayerController 0)))

(event Input|KeyboardEvents|N
  (params (Key :type Key%20Structure :default "None"))
  (bind _checkpoints (Variables|Default|GetCheckPoints))
  (bind _returnvalue (Utilities|Array|Length _checkpoints))
  (:Pressed
    (if (>= _returnvalue 2)
      (Variables|Default|SetCurrentIndex (Math|Integer|%(Integer) (+ (Variables|Default|GetCurrentIndex) 1) _returnvalue))
      (Transformation|SetActorLocation (Game|Player|GetPlayerPawn 0) (+ "0, 0,150.000000" (Transformation|GetWorldLocation (Variables|/Game/Blueprints/BP_CheckPoint.BP_CheckPoint_C|GetArrow (Utilities|Array|Get(acopy) _checkpoints (Variables|Default|GetCurrentIndex))))) false false)
      (Pawn|SetControlRotation (Game|GetPlayerController 0) (.rotation (Default|GetCheckPointRespawnTransform (Utilities|Array|Get(acopy) _checkpoints (Variables|Default|GetCurrentIndex))))))))

(fn ConstructionScript)