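; Rifle weapon Blueprint that fires a hitscan shot from the first player's camera view when StartFire runs.
; The trace start slides along the aim ray to the weapon's depth, skipping anything between camera and weapon.
; It runs on the Visibility channel out to WeaponRange from the camera.
; Any hit spawns an impact effect, and actors tagged Enemy also take damage.
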(event EventStartFire
  (bind (_location _rotation) (CallFunction|GetPlayerViewPoint))
  ;[1 1 1] CalculateAdjustedDirection
  (bind _output_get (Variables|Default|SetStartTrace _location))
  (bind _output_get_2 (Variables|Default|SetShootDir (Math|Rotator|GetRotationXVector _rotation)))
  ;[1 1 1] TraceShot
  (bind (_outhit _returnvalue) (Collision|LineTraceByChannel (+ (* _output_get_2 (Math|Vector|DotProduct (- (Transformation|GetActorLocation) _output_get) _output_get_2)) (Variables|Default|GetStartTrace)) (+ (Variables|Default|GetStartTrace) (* _output_get_2 (Variables|Default|GetWeaponRange))) "TraceTypeQuery1" false 0 "None"))
  (if _returnvalue
    (Utilities|FlowControl|Sequence
      (:then_0
        (Niagara|SpawnSystematLocation "/Game/ThirdParty/Stylized_VFX_StPack/Particles/UPDATE_1_2/P_Snaking_Hit_01.P_Snaking_Hit_01" (.ImpactPoint (Collision|BreakHitResult _outhit))))
      (:then_1
        (if (Actor|ActorHasTag (.HitActor (Collision|BreakHitResult _outhit)) "Enemy")
          (Game|Damage|ApplyDamage (.HitActor (Collision|BreakHitResult _outhit)) (Variables|Default|GetDamage) 0 self))))))

(fn ConstructionScript
  (|CallParentFunction))

(fn GetPlayerViewPoint
  (bind _output_get (LocalVariables|SetMyPlayerController (Game|GetPlayerController 0)))
  (if (Utilities|IsValid _output_get)
    (if (Utilities|IsValid (Variables|/Script/Engine.PlayerController|GetPlayerCameraManager (LocalVariables|GetMyPlayerController)))
      (return (Camera|GetCameraLocation (Variables|/Script/Engine.PlayerController|GetPlayerCameraManager (LocalVariables|GetMyPlayerController))) (Camera|GetCameraRotation (Variables|/Script/Engine.PlayerController|GetPlayerCameraManager (LocalVariables|GetMyPlayerController)))))))