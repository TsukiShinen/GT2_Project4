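; BP_LaunchGrenade_Weapon is a grenade launcher weapon that fires projectiles with a cooldown between shots.
; StartFire spawns a FirstPersonProjectile at the GrenadeSpawn socket, aimed along the weapon mesh's right vector, then calls DisableShoot.
; DisableShoot blocks firing and shows a reload widget, created at BeginPlay, until the DurationBetweenShoot delay ends.
; Switching weapons calls Disable, which runs the parent logic and removes the widget.
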(event Custom|DisableShoot
  (bind _reloadwidget (Variables|Default|GetReloadWidget))
  (Variables|Default|SetcanShoot false)
  (UserInterface|Viewport|AddtoViewport _reloadwidget 0)
  (Utilities|FlowControl|Delay (Variables|Default|GetDurationBetweenShoot))
  (Widget|RemovefromParent _reloadwidget)
  (Variables|Default|SetcanShoot true))

(event EventBeginPlay
  (bind _returnvalue (UserInterface|CreateWidget "/Game/Blueprints/Widgets/WGP_LaunchGrenadeReload.WGP_LaunchGrenadeReload_C"))
  (Variables|Default|SetReloadWidget _returnvalue))

(event EventDisable
  ;[1 1 1] Called when we switch weapons
  (|CallParentFunction)
  (Widget|RemovefromParent (Variables|Default|GetReloadWidget)))

(event EventStartFire
  (if (Variables|Default|GetcanShoot)
    (Game|SpawnActorfromClass "/Game/FirstPersonBP/Blueprints/FirstPersonProjectile.FirstPersonProjectile_C" (Math|Transform|MakeTransform (Transformation|GetSocketLocation (Variables|Default|GetSK_Weapon) "GrenadeSpawn") (Math|Conversions|RotationFromXVector (Math|Vector|GetRightVector (Variables|Default|GetSK_Weapon)))) "AdjustIfPossibleButDontSpawnIfColliding" 0 0) ; Spawn projectile
    (CallFunction|DisableShoot)))

(fn ConstructionScript
  (|CallParentFunction))