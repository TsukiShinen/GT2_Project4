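; BP_BaseWeapon is a base weapon Blueprint providing a common equip, fire and flashlight interface.
; Enable creates the configured UI widget and adds it to the viewport when DisplayHUD is set and the class is valid, and Disable removes and clears it.
; StartFire and StopFire are empty events, apparently left for child weapons to implement.
; TurnOnOffSpotLight toggles the attached spotlight's visibility through a stored flag.
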(event Custom|StartFire)

(event Custom|Enable
  (bind _weaponuiclass (Variables|Default|GetWeaponUIClass))
  (if (and (Variables|Default|GetbDisplayHUD) (Utilities|IsValidClass _weaponuiclass))
    (CallFunction|CreateWeaponWidget _weaponuiclass)))

(event Custom|StopFire)

(event Custom|Disable
  (Utilities|IsValid (Variables|Default|GetWeaponUI)
    (:Is%20Valid
      (Widget|RemovefromParent (Variables|Default|GetWeaponUI))
      (Variables|Default|SetWeaponUI 0))))

(event Custom|TurnOnOffSpotLight
  (bind _output_get (Variables|Default|SetspotLightVisibility (not (Variables|Default|GetspotLightVisibility))))
  (Rendering|SetVisibility (Variables|Default|GetSpotLight) _output_get false))

(fn ConstructionScript)

(fn CreateWeaponWidget
  (params (WidgetClass :type User%20Widget%20Class%20Reference))
  (bind _returnvalue (UserInterface|CreateWidget WidgetClass))
  (bind _output_get (Variables|Default|SetWeaponUI _returnvalue))
  (UserInterface|Viewport|AddtoViewport _output_get 0))