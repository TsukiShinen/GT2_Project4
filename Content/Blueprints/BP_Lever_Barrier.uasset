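; BP_Lever_Barrier is a lever-and-barrier obstacle that opens when the lever is triggered.
; Damage from the gun or rifle weapon, or a lever hit by any actor other than player pawn 0, triggers it.
; Both paths destroy the lever and disable barrier collision.
; A dynamic material is then created on the barrier, with unnamed vector and scalar parameter writes as placeholders for shader updates.
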(event OnComponentHit(Lever)
  (params (HitComponent :type Primitive%20Component%20Object%20Reference) (OtherActor :type Actor%20Object%20Reference) (OtherComp :type Primitive%20Component%20Object%20Reference) (NormalImpulse :type Vector :default "0, 0, 0") (Hit :type Hit%20Result%20Structure%20%28by%20ref%29))
  (bind _barrier (Variables|Default|GetBarrier))
  (if (!= OtherActor (Game|Player|GetPlayerPawn 0))
    (Components|DestroyComponent (Variables|Default|GetLever))
    (Collision|SetCollisionEnabled _barrier "NoCollision")
    ;[1 1 1] Si besoin d'envoyer des nouvelles data au shader de la barrière
    (bind _returnvalue (Rendering|Material|CreateDynamicMaterialInstance _barrier 0 (Rendering|Material|GetMaterial _barrier 0) "None" :!class /Script/Engine.PrimitiveComponent))
    (Rendering|Material|SetVectorParameterValue :self _returnvalue :!class /Script/Engine.MaterialInstanceDynamic)
    (Rendering|Material|SetScalarParameterValue _returnvalue "None" 0.0 :!class /Script/Engine.MaterialInstanceDynamic)))

(event Game|Damage|EventAnyDamage
  (params (Damage :type Float%20%28single-precision%29) (DamageType :type Damage%20Type%20Object%20Reference) (InstigatedBy :type Controller%20Object%20Reference) (DamageCauser :type Actor%20Object%20Reference))
  (bind _returnvalue (Utilities|GetClass DamageCauser))
  (bind _barrier (Variables|Default|GetBarrier))
  (if (or (== _returnvalue "/Game/Blueprints/Weapons/BP_Gun_Weapon.BP_Gun_Weapon_C") (== _returnvalue "/Game/Blueprints/Weapons/BP_Rifle_Weapon.BP_Rifle_Weapon_C"))
    (Components|DestroyComponent (Variables|Default|GetLever))
    (Collision|SetCollisionEnabled _barrier "NoCollision")
    ;[1 1 1] Si besoin d'envoyer des nouvelles data au shader de la barrière
    (bind _returnvalue_2 (Rendering|Material|CreateDynamicMaterialInstance _barrier 0 (Rendering|Material|GetMaterial _barrier 0) "None" :!class /Script/Engine.PrimitiveComponent))
    (Rendering|Material|SetVectorParameterValue :self _returnvalue_2 :!class /Script/Engine.MaterialInstanceDynamic)
    (Rendering|Material|SetScalarParameterValue _returnvalue_2 "None" 0.0 :!class /Script/Engine.MaterialInstanceDynamic)))

(fn ConstructionScript)