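; Blueprint function library with a helper that reports whether a character stands within a given nav mesh actor's area.
; IsCharacterOnNavMesh lowers the character's location by a fixed Z offset and tests that point against the actor's bounding box, returning false if either input is invalid.
; The test uses only the box bounds and does not query or project onto navigation data.
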(fn IsCharacteronNavMesh
  (params (Character :type Character%20Object%20Reference) (NavMesh :type Nav%20Mesh%20Bounds%20Volume%20Object%20Reference))
  (bind (_origin _boxextent) (Collision|GetActorBounds NavMesh false false))
  (if (and (Utilities|IsValid Character) (Utilities|IsValid NavMesh))
    (if (Math|Geometry|IsPointinBox (- (Transformation|GetActorLocation Character) "0, 0,100.000000") _origin _boxextent)
      (return true)
      (else
        (return false)))
    (else
      (return false))))