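; Enemy spawner actor that places a limited number of AI enemies around its location, then destroys itself.
; BeginPlay starts a looping timer at a configurable interval that spawns the configured enemy class at a random navigable point near the actor, raised slightly and ignoring collision.
; Each spawn decrements the remaining count, and the spawner destroys itself when it reaches zero.
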(event Custom|SpawnEnemy
  (AI|SpawnAIFromClass (Variables|Default|GetEnemyClass) 0 (+ (.RandomLocation (Class|NavigationSystemV1|GetRandomPointinNavigableRadius (Transformation|GetActorLocation) 1e+02 0 0)) "0, 0,100.000000") "0, 0, 0" true 0)
  (bind _result (Math|Integer|DecrementInt (Variables|Default|GetEnemiesToSpawn))
    (:%20%20
      (if (<= _result 0)
        (Actor|DestroyActor)))))

(event EventBeginPlay
  (Utilities|Time|SetTimerbyEvent (delegate Custom|SpawnEnemy) (Variables|Default|GetDurationBetweenSpawn) true))

(fn ConstructionScript)