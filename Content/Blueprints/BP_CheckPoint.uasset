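; BP_CheckPoint is a one-shot checkpoint actor that registers itself as the player's current respawn point.
; When the player pawn overlaps its Box, it passes itself to BP_MainGameMode's UpdateCheckPoint, then destroys the Box and checkpoint mesh while the actor remains.
; GetCheckPointRespawnTransform returns the world transform of an Arrow component, which marks the respawn location and facing.
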(event OnComponentBeginOverlap(Box)
  (params (OverlappedComponent :type Primitive%20Component%20Object%20Reference) (OtherActor :type Actor%20Object%20Reference) (OtherComp :type Primitive%20Component%20Object%20Reference) (OtherBodyIndex :type Integer) (bFromSweep :type Boolean) (SweepResult :type Hit%20Result%20Structure%20%28by%20ref%29))
  (if (== OtherActor (Game|Player|GetPlayerPawn 0))
    (bind _asbp_main_game_mode (Utilities|Casting|CastToBP_MainGameMode (Game|GetGameMode)))
    (Default|UpdateCheckPoint _asbp_main_game_mode self)
    (Components|DestroyComponent (Variables|Default|GetBox))
    (Components|DestroyComponent (Variables|Default|GetSM_CheckPoint))))

(fn ConstructionScript)

(fn GetCheckPointRespawnTransform
  (return (Transformation|GetWorldTransform (Variables|Default|GetArrow))))